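; AshbringerLitBP is a melee weapon that the player picks up and uses to damage actors.
; PickUp, when unattached, drops the equipped weapon at its own spot and attaches itself to the character's back socket.
; AttackReady and AttackNotReady toggle hitbox collision, which starts disabled.
; Box overlaps apply fixed damage and report it to AI damage sense, with a DoOnce and short delay limiting hit rate.
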(event `self.ReceiveBeginPlay`
  (`self.AttackNotReady`))

(event `self.PickUp`
  (bind _defaultsceneroot (`self.DefaultSceneRoot`))
  (bind _asbase_character (cast `/Game/ThirdPersonBP/Blueprints/Base_Character` (`GameplayStatics.GetPlayerCharacter` 0) :!pure true))
  (bind _equippedweapon (`/Game/ThirdPersonBP/Blueprints/ThirdPersonCharacter.EquippedWeapon` _asbase_character))
  (`/Engine/EditorBlueprintResources/StandardMacros.IsValid` (`self.GetAttachParentActor`)
    (:`Is Not Valid`
      (`/Engine/EditorBlueprintResources/StandardMacros.IsValid` _equippedweapon
        (:`Is Valid`
          (`self.K2_DetachFromActor` _equippedweapon "KeepRelative" "KeepRelative" "KeepRelative")
          (message `/Game/Ashbringers/WeaponPickupInterface.AttackNotReady` _equippedweapon)
          (`self.K2_SetActorLocationAndRotation` _equippedweapon (`SceneComponent.K2_GetComponentLocation` _defaultsceneroot) (`SceneComponent.K2_GetComponentRotation` _defaultsceneroot) false false))
        (:`Is Not Valid`
          _))
      (bind _output_get (set `/Game/ThirdPersonBP/Blueprints/ThirdPersonCharacter.EquippedWeapon` self _asbase_character))
      (`self.K2_AttachToComponent` (`Character.Mesh` _asbase_character) "weapon_back" "SnapToTarget" "SnapToTarget" "SnapToTarget")
      (message `/Game/Ashbringers/WeaponPickupInterface.AttackNotReady` _output_get))))

(event `self.Box.OnComponentBeginOverlap`
  (params (OverlappedComponent :type "PrimitiveComponent Object Reference") (OtherActor :type "Actor Object Reference") (OtherComp :type "PrimitiveComponent Object Reference") (OtherBodyIndex :type Integer) (bFromSweep :type Boolean) (SweepResult :type "HitResult Structure (by ref)"))
  (if (and (!= OtherActor self) (!= OtherActor (`self.GetAttachParentActor`)))
    (`/Engine/EditorBlueprintResources/StandardMacros.DoOnce` false :!label _label
      (:`Completed`
        (`GameplayStatics.ApplyDamage` OtherActor 10.0 (`self.GetInstigatorController`) (`self.GetAttachParentActor`) "/Script/Engine.DamageType")
        (`KismetSystemLibrary.PrintString` (`KismetSystemLibrary.GetDisplayName` OtherActor))
        (`AISense_Damage.ReportDamageEvent` OtherActor self 10.0 (`self.K2_GetActorLocation`) (`.ImpactPoint` (`GameplayStatics.BreakHitResult` SweepResult)) "Damage")
        (`KismetSystemLibrary.Delay` 0.4)
        (goto _label :!via `Reset`)))))

(event `self.AttackReady`
  (set `self.Attack Ready` true)
  (`PrimitiveComponent.SetCollisionEnabled` (`self.Box`) "QueryAndPhysics"))

(event `self.AttackNotReady`
  (set `self.Attack Ready` false)
  (`PrimitiveComponent.SetCollisionEnabled` (`self.Box`) "NoCollision"))

(fn `UserConstructionScript`)